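; Asteroid pawn for a quiz game that homes in on the player pawn and pauses to show a multiple-choice question when clicked.
; BeginPlay fills a QuestionWidget with the question and three alternatives and binds its buttons.
; Answers are matched by button text: correct adds score and destroys the asteroid, wrong deducts points and resumes the chase, both updating MyPlayerState.
; A fourth button closes the question unscored and resumes movement.
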(event `self.ReceiveBeginPlay`
  (bind _returnvalue (`|CreateWidget` "/Game/Blueprints/Actors/QuestionWidget.QuestionWidget_C" (`GameplayStatics.GetPlayerController` 0)))
  (set `self.QuestionWidget` _returnvalue)
  (`TextBlock.SetText` (`/Game/Blueprints/Actors/QuestionWidget.Question` (`self.QuestionWidget`)) (`KismetTextLibrary.Conv_StringToText` (`self.Question`)))
  (`TextBlock.SetText` (`/Game/Blueprints/Actors/QuestionWidget.TextBlock_0` (`self.QuestionWidget`)) (`KismetTextLibrary.Conv_StringToText` (`self.AlternativeA`)))
  (`TextBlock.SetText` (`/Game/Blueprints/Actors/QuestionWidget.TextBlock_1` (`self.QuestionWidget`)) (`KismetTextLibrary.Conv_StringToText` (`self.AlternativeB`)))
  (`TextBlock.SetText` (`/Game/Blueprints/Actors/QuestionWidget.TextBlock_2` (`self.QuestionWidget`)) (`KismetTextLibrary.Conv_StringToText` (`self.AlternativeC`)))
  (add `Button.OnClicked` (`/Game/Blueprints/Actors/QuestionWidget.Button_A` (`self.QuestionWidget`)) (delegate `OnClicked_Event_0`))
  (add `Button.OnClicked` (`/Game/Blueprints/Actors/QuestionWidget.Button_B` (`self.QuestionWidget`)) (delegate `OnClicked_Event_1`))
  (add `Button.OnClicked` (`/Game/Blueprints/Actors/QuestionWidget.Button_C` (`self.QuestionWidget`)) (delegate `OnClicked_Event_2`))
  (add `Button.OnClicked` (`/Game/Blueprints/Actors/QuestionWidget.Button_0` (`self.QuestionWidget`)) (delegate `OnClicked_Event_3`))
  (bind _asmy_player_state (cast `/Game/Blueprints/AllLevels/MyPlayerState` (`Controller.PlayerState` (`GameplayStatics.GetPlayerController` 0))))
  (set `self.Player` _asmy_player_state))

(event `OnClicked_Event_3`
  (`Widget.RemoveFromParent` (`self.QuestionWidget`))
  (set `self.Answer?` false)
  (set `self.VelocidadMov` 350.0))

(event `self.ReceiveTick`
  (params (DeltaSeconds :type "Float (single-precision)"))
  (bind _returnvalue (`self.K2_GetActorLocation`))
  ;[1 1 1] Movement
  (`self.K2_SetActorRelativeLocation` (+ _returnvalue (* (* (`KismetMathLibrary.Normal` (- (`self.K2_GetActorLocation` (`GameplayStatics.GetPlayerPawn` 0)) _returnvalue)) DeltaSeconds) (`self.VelocidadMov`)))))

(event `OnClicked_Event_0`
  (bind _player (`self.Player`))
  (bind _player_2 (`self.Player`))
  (bind _player_3 (`self.Player`))
  (bind _player_4 (`self.Player`))
  (if (`KismetStringLibrary.EqualEqual_StrStr` (`self.CorrectAlternative`) (`KismetTextLibrary.Conv_TextToString` (`TextBlock.GetText` (`/Game/Blueprints/Actors/QuestionWidget.TextBlock_0` (`self.QuestionWidget`)))))
    (set `/Game/Blueprints/AllLevels/MyPlayerState.Player_Score` (+ (`/Game/Blueprints/AllLevels/MyPlayerState.Player_Score` _player) 100) _player_4 :!label _label)
    (set `/Game/Blueprints/AllLevels/MyPlayerState.Answered` (+ (`/Game/Blueprints/AllLevels/MyPlayerState.Answered` _player) 1) _player_4)
    (set `/Game/Blueprints/AllLevels/MyPlayerState.Correct` (+ (`/Game/Blueprints/AllLevels/MyPlayerState.Correct` _player) 1) _player_4)
    (`self.K2_DestroyActor`)
    (else
      (set `/Game/Blueprints/AllLevels/MyPlayerState.Player_Score` (+ (`/Game/Blueprints/AllLevels/MyPlayerState.Player_Score` _player_2) -20) _player_3 :!label _label_2)
      (set `/Game/Blueprints/AllLevels/MyPlayerState.Answered` (+ (`/Game/Blueprints/AllLevels/MyPlayerState.Answered` _player_2) 1) _player_3)
      (set `self.VelocidadMov` 350.0)
      (set `self.Answer?` false)))
  (`Widget.RemoveFromParent` (`self.QuestionWidget`)))

(event `OnClicked_Event_1`
  (if (`KismetStringLibrary.EqualEqual_StrStr` (`self.CorrectAlternative`) (`KismetTextLibrary.Conv_TextToString` (`TextBlock.GetText` (`/Game/Blueprints/Actors/QuestionWidget.TextBlock_1` (`self.QuestionWidget`)))))
    (goto _label)
    (else
      (goto _label_2))))

(event `self.ReceiveActorOnClicked`
  (params (ButtonPressed :type "Key Structure"))
  ;[1 1 1] Question on Clicked
  (if (not (`self.Answer?`))
    (set `self.Answer?` true)
    (set `self.VelocidadMov` 0.0)
    (`UserWidget.AddToViewport` (`self.QuestionWidget`) 10)))

(event `OnClicked_Event_2`
  (if (`KismetStringLibrary.EqualEqual_StrStr` (`self.CorrectAlternative`) (`KismetTextLibrary.Conv_TextToString` (`TextBlock.GetText` (`/Game/Blueprints/Actors/QuestionWidget.TextBlock_2` (`self.QuestionWidget`)))))
    (goto _label)
    (else
      (goto _label_2))))

(fn `UserConstructionScript`)
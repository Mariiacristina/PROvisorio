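; Actor that spawns asteroid pawns inside a box volume while keeping their number in the world below a cap.
; Its SpawnAsteroid event counts existing AsteroidBP_Pawn actors and, if under MaxAsteroids, spawns one at a random point within SpawnVolume's bounds.
; Spawning adjusts position to avoid collisions but always succeeds, and nothing in this graph triggers the event itself.
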(event `SpawnAsteroid`
  (bind _spawn_volume (`self.Spawn Volume`))
  (bind _outactors (`GameplayStatics.GetAllActorsOfClass` "/Game/Blueprints/Actors/AsteroidBP_Pawn.AsteroidBP_Pawn_C"))
  (if (< (`KismetArrayLibrary.Array_Length` _outactors) (`self.MaxAsteroids`))
    (`|SpawnActorFromClass` "/Game/Blueprints/Actors/AsteroidBP_Pawn.AsteroidBP_Pawn_C" (`KismetMathLibrary.Conv_VectorToTransform` (`KismetMathLibrary.RandomPointInBoundingBox` (`SceneComponent.K2_GetComponentLocation` _spawn_volume) (`BoxComponent.GetScaledBoxExtent` _spawn_volume))) "AdjustIfPossibleButAlwaysSpawn" "OverrideRootScale" null null)))

(fn `UserConstructionScript`)